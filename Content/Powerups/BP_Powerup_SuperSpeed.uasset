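; BP_Powerup_SuperSpeed is a powerup that temporarily doubles the movement speed of the player who activates it.
; On activation it stores that player and sets their CharacterMovementComponent's MaxWalkSpeed to twice GetMaxSpeed, which depends on the current movement mode.
; On expiry it sets MaxWalkSpeed to half the then-current GetMaxSpeed if the player is still valid, then calls the parent's OnExpired.
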(event `self.OnActivated`
  (params (ActiveFor :type "Actor Object Reference"))
  (bind _returnvalue (`self.GetComponentByClass` (`self.Activated For Player`) "/Script/Engine.CharacterMovementComponent"))
  (set `self.Activated For Player` ActiveFor)
  (set `CharacterMovementComponent.MaxWalkSpeed` (* (`MovementComponent.GetMaxSpeed` _returnvalue) 2.0) _returnvalue))

(event `self.OnExpired`
  (bind _activated_for_player (`self.Activated For Player`))
  (bind _returnvalue (`self.GetComponentByClass` _activated_for_player "/Script/Engine.CharacterMovementComponent"))
  (`/Engine/EditorBlueprintResources/StandardMacros.IsValid` _activated_for_player
    (:`Is Valid`
      (set `CharacterMovementComponent.MaxWalkSpeed` (/ (`MovementComponent.GetMaxSpeed` _returnvalue) 2.0) _returnvalue))
    (:`Is Not Valid`
      _))
  (`parent.OnExpired`))

(fn `UserConstructionScript`)